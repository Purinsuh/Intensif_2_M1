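; BP_Laps is a lap-line actor for a racing game that counts laps when a vehicle pawn overlaps its trigger.
; Each overlap increments a single counter on the actor and writes the lap number to that vehicle's lap counter UI.
; When the counter equals three, it calls GetFinish on the racing GameInstance's widget and shows a "Finish" message there.
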(event `self.Trigger.OnComponentBeginOverlap`
  (params (OverlappedComponent :type "PrimitiveComponent Object Reference") (OtherActor :type "Actor Object Reference") (OtherComp :type "PrimitiveComponent Object Reference") (OtherBodyIndex :type Integer) (bFromSweep :type Boolean) (SweepResult :type "HitResult Structure (by ref)"))
  (bind _asvehicle_adv_pawn (cast `/Game/VehicleTemplate/Blueprints/VehicleAdvPawn` OtherActor))
  (`/Engine/EditorBlueprintResources/StandardMacros.IncrementInt` (`self.Laps`)
    (:`  `
      (`TextBlock.SetText` (`/Game/Camille/UI/WB_LapCounter.LapText` (`/Game/VehicleTemplate/Blueprints/VehicleAdvPawn.LapCounterUI` _asvehicle_adv_pawn)) (`|FormatText` "Lap {Lap Number}" (`self.Laps`)))
      (if (== (`self.Laps`) 3)
        (bind _asgi_racing_instance (cast `/Game/Camille/GI_RacingInstance` (`GameplayStatics.GetGameInstance`)))
        (bind _widget (`/Game/Camille/GI_RacingInstance.Widget` _asgi_racing_instance))
        (`/Game/Camille/UI/WB_Racing.GetFinish` _widget)
        (bind _messagetext (`/Game/Camille/UI/WB_Racing.MessageText` _widget))
        (`TextBlock.SetText` _messagetext "Finish")
        (`Widget.SetVisibility` _messagetext "Visible")))))

(fn `UserConstructionScript`)