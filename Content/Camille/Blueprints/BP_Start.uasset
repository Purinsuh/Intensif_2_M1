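; BP_Start is a start-line trigger that launches the racing timer when a VehicleAdvPawn overlaps it.
; A DoOnce-gated overlap creates the WB_Racing widget, stores it in GI_RacingInstance and adds it to the viewport.
; A looping 0.1-second Delay repeatedly calls the widget's Timer until its Finish flag is set, then resets the gate so the trigger can fire again.
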(event `self.Trigger.OnComponentBeginOverlap`
  (params (OverlappedComponent :type "PrimitiveComponent Object Reference") (OtherActor :type "Actor Object Reference") (OtherComp :type "PrimitiveComponent Object Reference") (OtherBodyIndex :type Integer) (bFromSweep :type Boolean) (SweepResult :type "HitResult Structure (by ref)"))
  (cast `/Game/VehicleTemplate/Blueprints/VehicleAdvPawn` OtherActor)
  (`/Engine/EditorBlueprintResources/StandardMacros.DoOnce` false :!label _label
    (:`Completed`
      (bind _returnvalue (`|CreateWidget` "/Game/Camille/UI/WB_Racing.WB_Racing_C"))
      (bind _asgi_racing_instance (cast `/Game/Camille/GI_RacingInstance` (`GameplayStatics.GetGameInstance`)))
      (bind _output_get (set `/Game/Camille/GI_RacingInstance.Widget` _returnvalue _asgi_racing_instance))
      (`UserWidget.AddToViewport` _returnvalue 0)
      (`/Game/Camille/UI/WB_Racing.Timer` _output_get :!label _label_2)
      (`KismetSystemLibrary.Delay` 0.1)
      (if (`/Game/Camille/UI/WB_Racing.Finish` _output_get)
        (goto _label :!via `Reset`)
        (else
          (goto _label_2))))))

(fn `UserConstructionScript`)