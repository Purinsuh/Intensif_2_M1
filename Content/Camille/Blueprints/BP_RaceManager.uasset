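; BP_RaceManager runs the race start, holding the player and AI cars still during a countdown.
; On BeginPlay it shows a WB_Countdown widget counting from three to "GO !", disables car movement, then re-enables it after a fixed delay.
; ToggleCarMovement applies the movement flag to three car arrays: player, Bowser AI and AirShip AI.
; The delay is timed independently of the widget rather than triggered by it.
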(event `self.ReceiveBeginPlay`
  (bind _returnvalue (`|CreateWidget` "/Game/Camille/UI/WB_Countdown.WB_Countdown_C"))
  (`/Game/Camille/UI/WB_Countdown.StartCountDown` _returnvalue 3 "GO !")
  (`UserWidget.AddToViewport` _returnvalue 0)
  (`self.ToggleCarMovement` false)
  (`KismetSystemLibrary.Delay` 4.0)
  (`self.ToggleCarMovement` true))

(fn `ToggleCarMovement`
  (params (MovementEnabled :type Boolean))
  (`|ExecutionSequence`
    (:`then_0`
      (for _array_element (`self.AICarsBowser`)
        (set `/Game/Camille/AI/VehicleAdvPawnAI.MovementEnabledAI` MovementEnabled _array_element)))
    (:`then_1`
      (for _array_element_2 (`self.PlayerCar`)
        (set `/Game/VehicleTemplate/Blueprints/VehicleAdvPawn.MovementEnabled` MovementEnabled _array_element_2)))
    (:`then_2`
      (for _array_element_3 (`self.AICarsAirShip`)
        (set `/Game/Camille/AI/VehicleAdvPawnAIV2.MovementEnabledAI` MovementEnabled _array_element_3)))))

(fn `UserConstructionScript`)