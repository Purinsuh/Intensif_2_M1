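; BP_MysteryBox is a pickup that grants a random power-up to player and AI vehicles driving into it.
; On box overlap, it fills the pawn's SlotItem with one of three random items and destroys itself, only if that slot is empty.
; Player pawns get a new WB_PowerUp widget on every overlap, even with a full slot; AI pawns call SetPowerUpMessage after a successful pickup.
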(event `self.ReceiveTick`
  (params (DeltaSeconds :type "Float (single-precision)")))

(event `self.Box.OnComponentBeginOverlap`
  (params (OverlappedComponent :type "PrimitiveComponent Object Reference") (OtherActor :type "Actor Object Reference") (OtherComp :type "PrimitiveComponent Object Reference") (OtherBodyIndex :type Integer) (bFromSweep :type Boolean) (SweepResult :type "HitResult Structure (by ref)"))
  (`|ExecutionSequence`
    (:`then_0`
      (bind _asvehicle_adv_pawn (cast `/Game/VehicleTemplate/Blueprints/VehicleAdvPawn` OtherActor))
      (bind _returnvalue (`|CreateWidget` "/Game/Camille/UI/WB_PowerUp.WB_PowerUp_C"))
      (`UserWidget.AddToViewport` _returnvalue 0)
      (if (== (`/Game/VehicleTemplate/Blueprints/VehicleAdvPawn.SlotItem` _asvehicle_adv_pawn) 0)
        (set `/Game/VehicleTemplate/Blueprints/VehicleAdvPawn.SlotItem` (`KismetMathLibrary.RandomIntegerInRange` 1 3) _asvehicle_adv_pawn)
        (`self.K2_DestroyActor`)))
    (:`then_1`
      (bind _asvehicle_adv_pawn_ai (cast `/Game/Camille/AI/VehicleAdvPawnAI` OtherActor))
      (if (== (`/Game/Camille/AI/VehicleAdvPawnAI.SlotItem` _asvehicle_adv_pawn_ai) 0)
        (set `/Game/Camille/AI/VehicleAdvPawnAI.SlotItem` (`KismetMathLibrary.RandomIntegerInRange` 1 3) _asvehicle_adv_pawn_ai)
        (`self.K2_DestroyActor`)
        (message `/Game/Camille/AI/BPI_Vehicle.SetPowerUp` _asvehicle_adv_pawn_ai)))))

(fn `UserConstructionScript`)