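; BP_RestartLevel is a trigger volume that sends the player's vehicle back when it enters the box, without reloading the level.
; On BeginPlay it caches the player pawn's starting transform.
; On overlap by that pawn, it casts to VehicleAdvPawn and calls Respawn if Checkpoints is above zero.
; Otherwise it teleports the pawn to the cached start transform.
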(event `self.ReceiveBeginPlay`
  (set `self.IntialTransform` (`self.GetTransform` (`GameplayStatics.GetPlayerPawn` 0))))

(event `self.Box.OnComponentBeginOverlap`
  (params (OverlappedComponent :type "PrimitiveComponent Object Reference") (OtherActor :type "Actor Object Reference") (OtherComp :type "PrimitiveComponent Object Reference") (OtherBodyIndex :type Integer) (bFromSweep :type Boolean) (SweepResult :type "HitResult Structure (by ref)"))
  (bind _returnvalue (`GameplayStatics.GetPlayerPawn` 0))
  (if (== OtherActor _returnvalue)
    (bind _asvehicle_adv_pawn (cast `/Game/VehicleTemplate/Blueprints/VehicleAdvPawn` _returnvalue))
    (if (> (`/Game/VehicleTemplate/Blueprints/VehicleAdvPawn.Checkpoints` _asvehicle_adv_pawn) 0)
      (`/Game/VehicleTemplate/Blueprints/VehicleAdvPawn.Respawn` _asvehicle_adv_pawn)
      (else
        (`self.K2_SetActorTransform` _returnvalue (`self.IntialTransform`) false true)))))

(fn `UserConstructionScript`)