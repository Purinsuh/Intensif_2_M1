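; Glitch box projectile actor for the car game that triggers a glitch malus when something overlaps it.
; On overlap it loops through the other actor's overlapping actors; a player pawn match with Shielded set deactivates the car's shield Niagara effect and blocks the glitch.
; Any other case calls VFXGlitchMalus on BP_PostProcess and plays a pickup sound.
; The box destroys itself inside the loop; a car-check debug loop is left unwired.
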(event `self.ReceiveActorBeginOverlap`
  (params (OtherActor :type "Actor Object Reference"))
  (for _array_element (`self.GetOverlappingActors` OtherActor null)
    (if (== _array_element (`GameplayStatics.GetPlayerPawn` 0))
      ;[1 1 1] Comment
      (bind _returnvalue (`GameplayStatics.GetActorOfClass` "/Game/Bosrah/Projectile/Bosrah_SportsCar_Pawn.Bosrah_SportsCar_Pawn_C"))
      (if (`/Game/Bosrah/Projectile/Bosrah_SportsCar_Pawn.Shielded` _returnvalue)
        (`ActorComponent.Deactivate` (`/Game/Bosrah/Projectile/Bosrah_SportsCar_Pawn.NS_Shield_0` _returnvalue))
        (`KismetSystemLibrary.PrintString` "Glitchbox failed")
        (else
          (bind _returnvalue_2 (`GameplayStatics.GetActorOfClass` "/Game/Bosrah/Projectile/BP_PostProcess.BP_PostProcess_C" :!label _label))
          (`/Game/Bosrah/Projectile/BP_PostProcess.VFX_GlitchMalus` _returnvalue_2)
          (`KismetSystemLibrary.PrintString` "glitchbox")
          (`GameplayStatics.PlaySound2D` "/Game/Bosrah/Son/SFX/BoxGet.BoxGet" 1.0 1.0 0.0 null null)))
      (else
        (goto _label)))
    (`self.K2_DestroyActor`)))

(fn `UserConstructionScript`)