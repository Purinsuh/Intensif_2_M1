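; BP_Camera is a cinematic camera actor that travels along a spline placed in the level.
; On BeginPlay it finds a BP_CmaeraSpline actor and starts the MoveObject timeline, with play rate derived from TimeToCompleteSeconds.
; Each update maps the timeline's Move value to distance along the spline and sets the actor's transform, sampling location in world space but rotation in local space.
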(event `self.ReceiveBeginPlay`
  (bind _returnvalue (`GameplayStatics.GetActorOfClass` "/Game/Bosrah/CInematic/BP_CmaeraSpline.BP_CmaeraSpline_C"))
  (set `self.SplineREF` _returnvalue)
  (`self.MoveOBJ`))

(event `MoveOBJ`
  (bind _spline (`/Game/Bosrah/CInematic/BP_CmaeraSpline.Spline` (`self.SplineREF`)))
  (`TimelineComponent.SetPlayRate` (`self.MoveObject`) (/ 1.0 (`self.TimeToComplete(Seconds)`)))
  (bind (_direction _move) (`Timeline|MoveObject`)
    (:`Update`
      (bind _returnvalue (`KismetMathLibrary.Lerp` 0.0 (`SplineComponent.GetSplineLength` (`/Game/Bosrah/CInematic/BP_CmaeraSpline.Spline` (`self.SplineREF`))) _move))
      (`self.K2_SetActorTransform` (`KismetMathLibrary.MakeTransform` (`SplineComponent.GetLocationAtDistanceAlongSpline` _spline _returnvalue "World") (`SplineComponent.GetRotationAtDistanceAlongSpline` _spline _returnvalue "Local"))))))

(fn `UserConstructionScript`)